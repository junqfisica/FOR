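; Basic melee enemy that chases the player character and dies when its life runs out.
; Tick drives AI MoveTo toward the player; overlapping the Collision component starts a looping damage timer and a timeline that moves the Cube as an attack animation.
; Incoming damage briefly stuns, applies knockback by offsetting the capsule, and reduces life.
; Death disables collision, tips the actor over by timeline, then destroys it after a delay.
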(event `self.ReceiveTick`
  (params (DeltaSeconds :type "Float (single-precision)"))
  (if (`self.isDead`)
    (`MovementComponent.StopMovementImmediately` (`self.CharacterMovement`))
    (else
      ;[1 1 1] Follow player
      (if (not (`self.isStun`))
        (`|AIMoveTo` self (0.0 0.0 0.0) (`self.target`) 5.0 true)))))

(event `self.Collision.OnComponentBeginOverlap`
  (params (OverlappedComponent :type "PrimitiveComponent Object Reference") (OtherActor :type "Actor Object Reference") (OtherComp :type "PrimitiveComponent Object Reference") (OtherBodyIndex :type Integer) (bFromSweep :type Boolean) (SweepResult :type "HitResult Structure (by ref)"))
  (cast `/Game/Blueprints/BP_TopDownCharacter` OtherActor)
  (`self.StartDamage`)
  (bind _returnvalue (`KismetSystemLibrary.K2_SetTimerDelegate` (delegate `StartDamage`) (`self.attackSpeed`) true))
  (set `self.applyDamageTimeHandler` _returnvalue)
  (`self.StartAttackAnimation` true))

(event `StartDamage`
  (`/Game/Blueprints/BP_TopDownCharacter.On Damage` (`self.target`) (`self.damage`) self (0.0 0.0 0.0)))

(event `self.Collision.OnComponentEndOverlap`
  (params (OverlappedComponent :type "PrimitiveComponent Object Reference") (OtherActor :type "Actor Object Reference") (OtherComp :type "PrimitiveComponent Object Reference") (OtherBodyIndex :type Integer))
  (bind _applydamagetimehandler (`self.applyDamageTimeHandler`))
  (cast `/Game/Blueprints/BP_TopDownCharacter` OtherActor)
  (if (`KismetSystemLibrary.K2_IsValidTimerHandle` _applydamagetimehandler)
    (`KismetSystemLibrary.K2_ClearAndInvalidateTimerHandle` _applydamagetimehandler)
    (`self.StartAttackAnimation` false)))

(event `removeStun`
  ;[1 1 1] Need some work
  (set `self.isStun` false))

(event `/Game/BPInterfaces/BPITakeDamage.On Damage`
  (params (value :type "Float (double-precision)") (perpetrator :type "Actor Object Reference") (impactForce :type "Vector Structure"))
  ;[1 1 1] Need some work
  (`|ExecutionSequence`
    (:`then_0`
      (set `self.isStun` true)
      (`MovementComponent.StopMovementImmediately` (`self.CharacterMovement`))
      (`SceneComponent.K2_AddWorldOffset` (`self.CapsuleComponent`) (* (`KismetMathLibrary.GetDirectionUnitVector` (`self.K2_GetActorLocation` perpetrator) (`self.K2_GetActorLocation` self)) impactForce) false false)
      (`KismetSystemLibrary.K2_SetTimerDelegate` (delegate `removeStun`) 0.2))
    (:`then_1`
      (bind _life (`self.TakeDamage` value))
      (bind _output_get (set `self.isDead` (<= _life 0.0)))
      (if _output_get
        (`self.onKillEnemy`)))))

(event `StartAttackAnimation`
  (params (bStart :type Boolean))
  (bind _startcubelocation (`self.startCubeLocation`))
  (if bStart
    (set `self.startCubeLocation` (`SceneComponent.RelativeLocation` (`self.Cube`)))
    (bind (_direction _alpha) (`Timeline|AttackAnimation` :!via `PlayFromStart` :!label _label)
      (:`Update`
        (`SceneComponent.K2_SetRelativeLocation` (`self.Cube`) (`KismetMathLibrary.VLerp` _startcubelocation (+ _startcubelocation (0.0 0.0 100.0)) _alpha) false false)))
    (else
      (`|ExecutionSequence`
        (:`then_0`
          (goto _label :!via `Stop`))
        (:`then_1`
          (`SceneComponent.K2_SetRelativeLocation` (`self.Cube`) (`self.startCubeLocation`) false false))))))

(event `onKillEnemy`
  (bind (_returnvalue_roll _returnvalue_pitch _returnvalue_yaw) (`KismetMathLibrary.BreakRotator` (`self.K2_GetActorRotation`)))
  (`PrimitiveComponent.SetCollisionEnabled` (`self.Collision`) "NoCollision")
  (bind (_direction _alpha) (`Timeline|DieAnimation` :!via `PlayFromStart`)
    (:`Update`
      (`self.K2_SetActorRotation` (`KismetMathLibrary.RLerp` (`self.K2_GetActorRotation`) (`KismetMathLibrary.MakeRotator` 0.0 89.0 _returnvalue_yaw) _alpha))
      (`KismetSystemLibrary.Delay` 2.0)
      (`self.K2_DestroyActor`))))

(event `self.ReceiveBeginPlay`
  (`|ExecutionSequence`
    (:`then_0`
      ;[1 1 1] Set the maxium speed for the enemy
      (set `CharacterMovementComponent.MaxWalkSpeed` (`self.speed`) (`self.CharacterMovement`)))
    (:`then_1`
      (bind _asbp_top_down_character (cast `/Game/Blueprints/BP_TopDownCharacter` (`GameplayStatics.GetPlayerCharacter` 0)))
      (set `self.target` _asbp_top_down_character))
    (:`then_2`
      (set `self.life` (`self.baseLife`)))))

(fn `TakeDamage`
  (params (value :type "Float (double-precision)"))
  (returns (life :type "Float (double-precision)"))
  (bind _output_get (set `self.life` (`KismetMathLibrary.FMax` (- (`self.life`) value))))
  (return _output_get))

(fn `UserConstructionScript`)